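; Player character Blueprint that tracks health and puts a HUD_Bars widget on screen at BeginPlay.
; Two input actions change CurrentHealth by a fixed step without clamping, with inverted naming: Lebenplus subtracts and Lebenminus adds.
; The HudStates function exposes CurrentHealth and MaxHealth, apparently for the HUD to read.
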(event EventBeginPlay
  (bind _returnvalue (UserInterface|CreateWidget "/Game/HUD/HUD_Bars.HUD_Bars_C"))
  (UserInterface|Viewport|AddtoViewport _returnvalue 0))

(event Collision|EventActorBeginOverlap
  (params (OtherActor :type Actor%20Object%20Reference)))

(event EventTick
  (params (DeltaSeconds :type Float%20%28single-precision%29)))

(event Input|ActionEvents|InputActionLebenplus
  (params (Key :type Key%20Structure :default "AnyKey"))
  (:Pressed
    (Variables|Default|SetCurrentHealth (- (Variables|Default|GetCurrentHealth) 1e+01))))

(event Input|ActionEvents|InputActionLebenminus
  (params (Key :type Key%20Structure :default "AnyKey"))
  (:Pressed
    (Variables|Default|SetCurrentHealth (+ (Variables|Default|GetCurrentHealth) 1e+01))))

(fn ConstructionScript)

(fn HudStates
  (return (Variables|Default|GetCurrentHealth) (Variables|Default|GetMaxHealth)))