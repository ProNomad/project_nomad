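; BP_CharactorRecorder is a character stand-in, apparently for a HUD scene-capture preview, that mirrors equipped items on its skeletal mesh.
; On BeginPlay it passes a reference to itself to the player's Character_Controller.
; EquipItem switches on item slot, replacing that slot's actor with a spawned armor or weapon snapped to its socket, with hands and feet spawning pairs.
; UnequipItem destroys the slot's actors.
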(event EventBeginPlay
  (bind _ascharacter_controller (Utilities|Casting|CastToCharacter_Controller (Game|GetPlayerCharacter 0)))
  (Class|BPIRecorderComm|PassReference(Message) _ascharacter_controller self))

(event EventEquipItem
  (params (ItemInfo :type F%20Item%20Info%20Structure))
  (CallFunction|AttachItem ItemInfo))

(event EventUnequipItem
  (params (ItemInfo :type F%20Item%20Info%20Structure))
  (CallFunction|UnattachItem ItemInfo))

(fn ConstructionScript)

(fn AttachItem
  (params (ItemInfo :type F%20Item%20Info%20Structure))
  (bind (_itemclass _itemslot) (Utilities|Struct|BreakFItemInfo ItemInfo))
  (switch Utilities|FlowControl|Switch|SwitchonEquipSlot _itemslot
    (:NewEnumerator1
      (Utilities|IsValid (Variables|Default|GetHeadItem)
        (:Is%20Valid
          (Actor|DestroyActor (Variables|Default|GetHeadItem)))
        (:Is%20Not%20Valid
          _))
      (bind _returnvalue (Game|SpawnActorfromClass _itemclass (Transformation|GetActorTransform) "AlwaysSpawn" 0 0))
      (bind _output_get (Variables|Default|SetHeadItem _returnvalue))
      (bind _asbp_base_armor (Utilities|Casting|CastToBP_BaseArmor _output_get))
      (Transformation|AttachComponentToComponent _asbp_base_armor (Variables|Default|GetSkeletalMesh) (.MainAttachPoint (Utilities|Struct|BreakFArmorInfo (Variables|/Game/Interactables/BP_BaseArmor.BP_BaseArmor_C|GetArmorInfo _asbp_base_armor))) "SnapToTarget" "SnapToTarget" "SnapToTarget" true)
      (Collision|SetActorEnableCollision _asbp_base_armor false)
      (Physics|SetSimulatePhysics (Variables|/Game/Interactables/BP_BaseInteractable.BP_BaseInteractable_C|GetInteractableMesh _asbp_base_armor) false))
    (:NewEnumerator2
      (Utilities|IsValid (Variables|Default|GetTorsoItem)
        (:Is%20Valid
          (Actor|DestroyActor (Variables|Default|GetTorsoItem)))
        (:Is%20Not%20Valid
          _))
      (bind _returnvalue_2 (Game|SpawnActorfromClass _itemclass (Transformation|GetActorTransform) "AlwaysSpawn" 0 0))
      (bind _output_get_2 (Variables|Default|SetTorsoItem _returnvalue_2))
      (bind _asbp_base_armor_2 (Utilities|Casting|CastToBP_BaseArmor _output_get_2))
      (Transformation|AttachComponentToComponent _asbp_base_armor_2 (Variables|Default|GetSkeletalMesh) (.MainAttachPoint (Utilities|Struct|BreakFArmorInfo (Variables|/Game/Interactables/BP_BaseArmor.BP_BaseArmor_C|GetArmorInfo _asbp_base_armor_2))) "SnapToTarget" "SnapToTarget" "SnapToTarget" true)
      (Collision|SetActorEnableCollision _asbp_base_armor_2 false)
      (Physics|SetSimulatePhysics (Variables|/Game/Interactables/BP_BaseInteractable.BP_BaseInteractable_C|GetInteractableMesh _asbp_base_armor_2) false))
    (:NewEnumerator3
      (Utilities|IsValid (Variables|Default|GetRightArmItem)
        (:Is%20Valid
          (Actor|DestroyActor (Variables|Default|GetRightArmItem)))
        (:Is%20Not%20Valid
          _))
      (bind _returnvalue_3 (Game|SpawnActorfromClass _itemclass (Transformation|GetActorTransform) "AlwaysSpawn" 0 0))
      (bind _output_get_3 (Variables|Default|SetRightArmItem _returnvalue_3))
      (bind _asbp_base_armor_3 (Utilities|Casting|CastToBP_BaseArmor _output_get_3))
      (Transformation|AttachComponentToComponent _asbp_base_armor_3 (Variables|Default|GetSkeletalMesh) (.MainAttachPoint (Utilities|Struct|BreakFArmorInfo (Variables|/Game/Interactables/BP_BaseArmor.BP_BaseArmor_C|GetArmorInfo _asbp_base_armor_3))) "SnapToTarget" "SnapToTarget" "SnapToTarget" true)
      (Collision|SetActorEnableCollision _asbp_base_armor_3 false)
      (Utilities|IsValid (Variables|Default|GetLeftArmItem)
        (:Is%20Valid
          (Actor|DestroyActor (Variables|Default|GetLeftArmItem)))
        (:Is%20Not%20Valid
          _))
      (bind _returnvalue_4 (Game|SpawnActorfromClass _itemclass (Transformation|GetActorTransform) "AlwaysSpawn" 0 0))
      (bind _output_get_4 (Variables|Default|SetLeftArmItem _returnvalue_4))
      (bind _asbp_base_armor_4 (Utilities|Casting|CastToBP_BaseArmor _output_get_4))
      (Transformation|AttachComponentToComponent _asbp_base_armor_4 (Variables|Default|GetSkeletalMesh) (.LeftAttachPoint (Utilities|Struct|BreakFArmorInfo (Variables|/Game/Interactables/BP_BaseArmor.BP_BaseArmor_C|GetArmorInfo _asbp_base_armor_4))) "SnapToTarget" "SnapToTarget" "SnapToTarget" true)
      (Collision|SetActorEnableCollision _asbp_base_armor_4 false)
      (Physics|SetSimulatePhysics (Variables|/Game/Interactables/BP_BaseInteractable.BP_BaseInteractable_C|GetInteractableMesh _asbp_base_armor_4) false))
    (:NewEnumerator4
      (Utilities|IsValid (Variables|Default|GetLegsItem)
        (:Is%20Valid
          (Actor|DestroyActor (Variables|Default|GetLegsItem)))
        (:Is%20Not%20Valid
          _))
      (bind _returnvalue_5 (Game|SpawnActorfromClass _itemclass (Transformation|GetActorTransform) "AlwaysSpawn" 0 0))
      (bind _output_get_5 (Variables|Default|SetLegsItem _returnvalue_5))
      (bind _asbp_base_armor_5 (Utilities|Casting|CastToBP_BaseArmor _output_get_5))
      (Transformation|AttachComponentToComponent _asbp_base_armor_5 (Variables|Default|GetSkeletalMesh) (.RightAttachPoint (Utilities|Struct|BreakFArmorInfo (Variables|/Game/Interactables/BP_BaseArmor.BP_BaseArmor_C|GetArmorInfo _asbp_base_armor_5))) "SnapToTarget" "SnapToTarget" "SnapToTarget" true)
      (Collision|SetActorEnableCollision _asbp_base_armor_5 false)
      (Physics|SetSimulatePhysics (Variables|/Game/Interactables/BP_BaseInteractable.BP_BaseInteractable_C|GetInteractableMesh _asbp_base_armor_5) false))
    (:NewEnumerator5
      (Utilities|IsValid (Variables|Default|GetRightFeetItem)
        (:Is%20Valid
          (Actor|DestroyActor (Variables|Default|GetRightFeetItem)))
        (:Is%20Not%20Valid
          _))
      (bind _returnvalue_6 (Game|SpawnActorfromClass _itemclass (Transformation|GetActorTransform) "AlwaysSpawn" 0 0))
      (bind _output_get_6 (Variables|Default|SetRightFeetItem _returnvalue_6))
      (bind _asbp_base_armor_6 (Utilities|Casting|CastToBP_BaseArmor _output_get_6))
      (Transformation|AttachComponentToComponent _asbp_base_armor_6 (Variables|Default|GetSkeletalMesh) (.RightAttachPoint (Utilities|Struct|BreakFArmorInfo (Variables|/Game/Interactables/BP_BaseArmor.BP_BaseArmor_C|GetArmorInfo _asbp_base_armor_6))) "SnapToTarget" "SnapToTarget" "SnapToTarget" true)
      (Collision|SetActorEnableCollision _asbp_base_armor_6 false)
      (Utilities|IsValid (Variables|Default|GetLeftFeetItem)
        (:Is%20Valid
          (Actor|DestroyActor (Variables|Default|GetLeftFeetItem)))
        (:Is%20Not%20Valid
          _))
      (bind _returnvalue_7 (Game|SpawnActorfromClass _itemclass (Transformation|GetActorTransform) "AlwaysSpawn" 0 0))
      (bind _output_get_7 (Variables|Default|SetLeftFeetItem _returnvalue_7))
      (bind _asbp_base_armor_7 (Utilities|Casting|CastToBP_BaseArmor _output_get_7))
      (Transformation|AttachComponentToComponent _asbp_base_armor_7 (Variables|Default|GetSkeletalMesh) (.LeftAttachPoint (Utilities|Struct|BreakFArmorInfo (Variables|/Game/Interactables/BP_BaseArmor.BP_BaseArmor_C|GetArmorInfo _asbp_base_armor_7))) "SnapToTarget" "SnapToTarget" "SnapToTarget" true)
      (Collision|SetActorEnableCollision _asbp_base_armor_7 false)
      (Physics|SetSimulatePhysics (Variables|/Game/Interactables/BP_BaseInteractable.BP_BaseInteractable_C|GetInteractableMesh _asbp_base_armor_7) false))
    (:NewEnumerator6
      (Utilities|IsValid (Variables|Default|GetRightHandItem)
        (:Is%20Valid
          (Actor|DestroyActor (Variables|Default|GetRightHandItem)))
        (:Is%20Not%20Valid
          _))
      (bind _returnvalue_8 (Game|SpawnActorfromClass _itemclass (Transformation|GetActorTransform) "AlwaysSpawn" 0 0))
      (bind _output_get_8 (Variables|Default|SetRightHandItem _returnvalue_8))
      (bind _asbp_base_weapon (Utilities|Casting|CastToBP_BaseWeapon _output_get_8))
      (Transformation|AttachComponentToComponent _asbp_base_weapon (Variables|Default|GetSkeletalMesh) (Utilities|Struct|BreakFWeaponInfo (Variables|/Game/Interactables/BP_BaseWeapon.BP_BaseWeapon_C|GetWeaponInfo _asbp_base_weapon)) "SnapToTarget" "SnapToTarget" "SnapToTarget" true)
      (Collision|SetActorEnableCollision _asbp_base_weapon false)
      (Physics|SetSimulatePhysics (Variables|/Game/Interactables/BP_BaseInteractable.BP_BaseInteractable_C|GetInteractableMesh _asbp_base_weapon) false))
    (:NewEnumerator7
      (Utilities|IsValid (Variables|Default|GetLeftHandItem)
        (:Is%20Valid
          (Actor|DestroyActor (Variables|Default|GetLeftHandItem)))
        (:Is%20Not%20Valid
          _))
      (bind _returnvalue_9 (Game|SpawnActorfromClass _itemclass (Transformation|GetActorTransform) "AlwaysSpawn" 0 0))
      (bind _output_get_9 (Variables|Default|SetLeftHandItem _returnvalue_9))
      (bind _asbp_base_weapon_2 (Utilities|Casting|CastToBP_BaseWeapon _output_get_9))
      (Transformation|AttachComponentToComponent _asbp_base_weapon_2 (Variables|Default|GetSkeletalMesh) (Utilities|Struct|BreakFWeaponInfo (Variables|/Game/Interactables/BP_BaseWeapon.BP_BaseWeapon_C|GetWeaponInfo _asbp_base_weapon_2)) "SnapToTarget" "SnapToTarget" "SnapToTarget" true)
      (Collision|SetActorEnableCollision _asbp_base_weapon_2 false)
      (Physics|SetSimulatePhysics (Variables|/Game/Interactables/BP_BaseInteractable.BP_BaseInteractable_C|GetInteractableMesh _asbp_base_weapon_2) false))
    (:NewEnumerator8
      (Utilities|IsValid (Variables|Default|GetSchulterItem)
        (:Is%20Valid
          (Actor|DestroyActor (Variables|Default|GetSchulterItem)))
        (:Is%20Not%20Valid
          _))
      (bind _returnvalue_10 (Game|SpawnActorfromClass _itemclass (Transformation|GetActorTransform) "AlwaysSpawn" 0 0))
      (bind _output_get_10 (Variables|Default|SetSchulterItem _returnvalue_10))
      (bind _asbp_base_armor_8 (Utilities|Casting|CastToBP_BaseArmor _output_get_10))
      (Transformation|AttachComponentToComponent _asbp_base_armor_8 (Variables|Default|GetSkeletalMesh) (.MainAttachPoint (Utilities|Struct|BreakFArmorInfo (Variables|/Game/Interactables/BP_BaseArmor.BP_BaseArmor_C|GetArmorInfo _asbp_base_armor_8))) "SnapToTarget" "SnapToTarget" "SnapToTarget" true)
      (Collision|SetActorEnableCollision _asbp_base_armor_8 false)
      (Physics|SetSimulatePhysics (Variables|/Game/Interactables/BP_BaseInteractable.BP_BaseInteractable_C|GetInteractableMesh _asbp_base_armor_8) false))
    (:NewEnumerator9
      (Utilities|IsValid (Variables|Default|GetUmhangItem)
        (:Is%20Valid
          (Actor|DestroyActor (Variables|Default|GetUmhangItem)))
        (:Is%20Not%20Valid
          _))
      (bind _returnvalue_11 (Game|SpawnActorfromClass _itemclass (Transformation|GetActorTransform) "AlwaysSpawn" 0 0))
      (bind _output_get_11 (Variables|Default|SetUmhangItem _returnvalue_11))
      (bind _asbp_base_armor_9 (Utilities|Casting|CastToBP_BaseArmor _output_get_11))
      (Transformation|AttachComponentToComponent _asbp_base_armor_9 (Variables|Default|GetSkeletalMesh) (.MainAttachPoint (Utilities|Struct|BreakFArmorInfo (Variables|/Game/Interactables/BP_BaseArmor.BP_BaseArmor_C|GetArmorInfo _asbp_base_armor_9))) "SnapToTarget" "SnapToTarget" "SnapToTarget" true)
      (Collision|SetActorEnableCollision _asbp_base_armor_9 false)
      (Physics|SetSimulatePhysics (Variables|/Game/Interactables/BP_BaseInteractable.BP_BaseInteractable_C|GetInteractableMesh _asbp_base_armor_9) false))
    (:NewEnumerator10
      (Utilities|IsValid (Variables|Default|GetRingItem)
        (:Is%20Valid
          (Actor|DestroyActor (Variables|Default|GetRingItem)))
        (:Is%20Not%20Valid
          _))
      (bind _returnvalue_12 (Game|SpawnActorfromClass _itemclass (Transformation|GetActorTransform) "AlwaysSpawn" 0 0))
      (bind _output_get_12 (Variables|Default|SetRingItem _returnvalue_12))
      (bind _asbp_base_armor_10 (Utilities|Casting|CastToBP_BaseArmor _output_get_12))
      (Transformation|AttachComponentToComponent _asbp_base_armor_10 (Variables|Default|GetSkeletalMesh) (.MainAttachPoint (Utilities|Struct|BreakFArmorInfo (Variables|/Game/Interactables/BP_BaseArmor.BP_BaseArmor_C|GetArmorInfo _asbp_base_armor_10))) "SnapToTarget" "SnapToTarget" "SnapToTarget" true)
      (Collision|SetActorEnableCollision _asbp_base_armor_10 false)
      (Physics|SetSimulatePhysics (Variables|/Game/Interactables/BP_BaseInteractable.BP_BaseInteractable_C|GetInteractableMesh _asbp_base_armor_10) false))
    (:NewEnumerator11
      (Utilities|IsValid (Variables|Default|GetAmuletItem)
        (:Is%20Valid
          (Actor|DestroyActor (Variables|Default|GetAmuletItem)))
        (:Is%20Not%20Valid
          _))
      (bind _returnvalue_13 (Game|SpawnActorfromClass _itemclass (Transformation|GetActorTransform) "AlwaysSpawn" 0 0))
      (bind _output_get_13 (Variables|Default|SetAmuletItem _returnvalue_13))
      (bind _asbp_base_armor_11 (Utilities|Casting|CastToBP_BaseArmor _output_get_13))
      (Transformation|AttachComponentToComponent _asbp_base_armor_11 (Variables|Default|GetSkeletalMesh) (.MainAttachPoint (Utilities|Struct|BreakFArmorInfo (Variables|/Game/Interactables/BP_BaseArmor.BP_BaseArmor_C|GetArmorInfo _asbp_base_armor_11))) "SnapToTarget" "SnapToTarget" "SnapToTarget" true)
      (Collision|SetActorEnableCollision _asbp_base_armor_11 false)
      (Physics|SetSimulatePhysics (Variables|/Game/Interactables/BP_BaseInteractable.BP_BaseInteractable_C|GetInteractableMesh _asbp_base_armor_11) false))
    (:NewEnumerator12
      (Utilities|IsValid (Variables|Default|GetGürtelItem)
        (:Is%20Valid
          (Actor|DestroyActor (Variables|Default|GetGürtelItem)))
        (:Is%20Not%20Valid
          _))
      (bind _returnvalue_14 (Game|SpawnActorfromClass _itemclass (Transformation|GetActorTransform) "AlwaysSpawn" 0 0))
      (bind _output_get_14 (Variables|Default|SetGürtelItem _returnvalue_14))
      (bind _asbp_base_armor_12 (Utilities|Casting|CastToBP_BaseArmor _output_get_14))
      (Transformation|AttachComponentToComponent _asbp_base_armor_12 (Variables|Default|GetSkeletalMesh) (.MainAttachPoint (Utilities|Struct|BreakFArmorInfo (Variables|/Game/Interactables/BP_BaseArmor.BP_BaseArmor_C|GetArmorInfo _asbp_base_armor_12))) "SnapToTarget" "SnapToTarget" "SnapToTarget" true)
      (Collision|SetActorEnableCollision _asbp_base_armor_12 false)
      (Physics|SetSimulatePhysics (Variables|/Game/Interactables/BP_BaseInteractable.BP_BaseInteractable_C|GetInteractableMesh _asbp_base_armor_12) false))))

(fn UnattachItem
  (params (Iteminfo :type F%20Item%20Info%20Structure))
  (switch Utilities|FlowControl|Switch|SwitchonEquipSlot (Utilities|Struct|BreakFItemInfo Iteminfo)
    (:NewEnumerator1
      (Actor|DestroyActor (Variables|Default|GetHeadItem)))
    (:NewEnumerator2
      (Actor|DestroyActor (Variables|Default|GetTorsoItem)))
    (:NewEnumerator3
      (Actor|DestroyActor (Variables|Default|GetRightArmItem)))
    (:NewEnumerator4
      (Actor|DestroyActor (Variables|Default|GetLegsItem)))
    (:NewEnumerator5
      (Actor|DestroyActor (Variables|Default|GetRightFeetItem)))
    (:NewEnumerator6
      (Actor|DestroyActor (Variables|Default|GetRightHandItem)))
    (:NewEnumerator7
      (Actor|DestroyActor (Variables|Default|GetLeftHandItem)))
    (:NewEnumerator8
      (Actor|DestroyActor (Variables|Default|GetSchulterItem)))
    (:NewEnumerator9
      (Actor|DestroyActor (Variables|Default|GetUmhangItem)))
    (:NewEnumerator10
      (Actor|DestroyActor (Variables|Default|GetRingItem)))
    (:NewEnumerator11
      (Actor|DestroyActor (Variables|Default|GetAmuletItem)))
    (:NewEnumerator12
      (Actor|DestroyActor (Variables|Default|GetGürtelItem)))))